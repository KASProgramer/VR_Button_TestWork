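; Physical push button actor that fills an on-screen progress bar with repeated presses, then raises a TV.
; An overlapping component drives the button's clamped X offset; ending its Box overlap lets the button interpolate back.
; Tick counts each full press once, re-arms at rest, and starts the TV lift when the bar is full, removing the widget.
; Movie.OpenSource runs every tick the TV is not moving, including before the lift.
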(event OnComponentBeginOverlap(Button)
  (params (OverlappedComponent :type Primitive%20Component%20Object%20Reference) (OtherActor :type Actor%20Object%20Reference) (OtherComp :type Primitive%20Component%20Object%20Reference) (OtherBodyIndex :type Integer) (bFromSweep :type Boolean) (SweepResult :type Hit%20Result%20Structure%20%28by%20ref%29))
  (bind _umg (Variables|Default|GetUMG))
  ;[1 1 1] Проверяем соприкасается кнопка с игровым объектом или нет. Также, в этот момент выводим прогрессбар на экран, если его нет.
  (Utilities|IsValid (Variables|Default|GetgoPrimittive)
    (:Is%20Not%20Valid
      (Variables|Default|SetgoPrimittive OtherComp)
      (Variables|Default|SetgoPrimittiveLocation (Transformation|GetWorldLocation OtherComp))
      (if (not (UserInterface|Viewport|IsinViewport _umg))
        (UserInterface|Viewport|AddtoViewport _umg 0)))))

(event OnComponentEndOverlap(Box)
  (params (OverlappedComponent :type Primitive%20Component%20Object%20Reference) (OtherActor :type Actor%20Object%20Reference) (OtherComp :type Primitive%20Component%20Object%20Reference) (OtherBodyIndex :type Integer))
  ;[1 1 1] Проверяем что столкновения нет и деинециализируем объект с которым было столкновение
  (if (== OtherComp (Variables|Default|GetgoPrimittive))
    (Variables|Default|SetgoPrimittive 0)))

(event EventBeginPlay
  ;[1 1 1] Инициализируем виджет, в котором реализован прогресс бар.
  (bind _returnvalue (UserInterface|CreateWidget "/Game/Button/GUI/ButtonPressProgress.ButtonPressProgress_C"))
  (Variables|Default|SetUMG _returnvalue))

(event EventTick
  (params (DeltaSeconds :type Float%20%28single-precision%29))
  (bind _tv (Variables|Default|GetTV))
  (bind _button (Variables|Default|GetButton))
  (bind _relativelocation (Variables|/Script/Engine.SceneComponent|GetRelativeLocation _tv))
  ;[1 1 1] Запускаем проверки в разных потоках
  (Utilities|FlowControl|Sequence
    (:then_0
      ;[1 1 1] Есть ли нажатие на кнопку?
      (Utilities|IsValid (Variables|Default|GetgoPrimittive)
        (:Is%20Valid
          ;[1 1 1] Если нажатие произошло, узнаем дистанцию на которую прошел объект с момента нажатия. И на нее же смещаем кнопку. (лимит смещения кнопки от 0 до 5)
          (Transformation|SetRelativeLocation (Variables|Default|GetButton) (Math|Vector|MakeVector (Math|Float|Clamp(Float) (* (- (.x (Variables|Default|GetgoPrimittiveLocation)) (.x (Transformation|GetWorldLocation (Variables|Default|GetgoPrimittive)))) -1.0) 0.0 5.0) 0.0 0.0) false false)
          ;[1 1 1] Если кнопка нажата полностью (ее х координата == 5), и IsControl (по умолчанию true) - отвечает за возможность поднятия значения в прогресс баре. Следом поднимаем значение (вызвав функцию из канваса), после чего IsControlменяем на false, чтобы дождаться, пока кнопка не вернеться в изначальное положение. После чего IsControl станет true и мы сможем снова поднимать значение на шкале прогрессбара
          (if (== (.x (Variables|/Script/Engine.SceneComponent|GetRelativeLocation (Variables|Default|GetButton))) 5.0)
            (if (Variables|Default|GetisControl)
              (Default|ProgressBarCountPlus (Variables|Default|GetUMG))
              (Variables|Default|SetisControl false))))
        (:Is%20Not%20Valid
          ;[1 1 1] Возврат кнопки в начальное положение (с текущего к координатам 0,0,0).
          (Transformation|SetRelativeLocation _button (Math|Interpolation|VInterpTo (Variables|/Script/Engine.SceneComponent|GetRelativeLocation _button) "0, 0, 0" DeltaSeconds 1e+01) false false))))
    (:then_1
      ;[1 1 1] Проверка "Вернулась ли кнопка в изначальное положение"
      (if (== (.x (Variables|/Script/Engine.SceneComponent|GetRelativeLocation (Variables|Default|GetButton))) 0.0)
        (Variables|Default|SetisControl true)
        ;[1 1 1] Проверка, заполнен ли прогресс бар полностью
        (if (>= (Variables|/Script/UMG.ProgressBar|GetPercent (Variables|/Game/Button/GUI/ButtonPressProgress.ButtonPressProgress_C|GetProgressBar_185 (Variables|Default|GetUMG))) 1.0)
          (Variables|Default|SetMove_TV true))))
    (:then_2
      ;[1 1 1] Поднимаем теливизор, если прогресс бар был заполнен
      (if (Variables|Default|GetMove_TV)
        (if (< (.z _relativelocation) 2e+02)
          (Transformation|SetRelativeLocation _tv (Math|Vector|MakeVector (.x _relativelocation) (.y _relativelocation) (+ (.z _relativelocation) 1.0)) false false)
          (Widget|RemovefromParent (Variables|Default|GetUMG))
          (else
            (Variables|Default|SetMove_TV false)))
        (else
          ;[1 1 1] Включаем телевизор, когда тот поднимется
          (Media|MediaPlayer|OpenSource (Variables|Default|GetMovie) "/Game/Button/Movie/TW_Video.TW_Video"))))))

(fn ConstructionScript)